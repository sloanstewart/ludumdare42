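; Vegan enemy Blueprint that chases what it sees, hurts what it touches and can be killed by damage.
; PawnSensing triggers an AI MoveTo aimed at the player controller, and any hit applies touch damage to the other actor.
; Damage lowers Health; at zero or below the mesh ragdolls, the capsule is destroyed and the FirstPersonCharacter's kill count updates.
; The body is removed after a delay.
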(event OnSeePawn(PawnSensing)
  (params (Pawn :type Pawn%20Object%20Reference))
  ;[1 1 1] See Player & Move Towards
  (AI|AIMoveTo (Class|PawnMovementComponent|GetPawnOwner (Variables|Character|GetCharacterMovement)) "0, 0, 0" (Game|GetPlayerController 0) 5.0 false))

(event Custom|EnemyKilled
  (bind _asfirst_person_character (Utilities|Casting|CastToFirstPersonCharacter (Game|GetPlayerCharacter 0)))
  (Default|UpdateKillCount _asfirst_person_character))

(event Collision|EventHit
  (params (MyComp :type Primitive%20Component%20Object%20Reference) (Other :type Actor%20Object%20Reference) (OtherComp :type Primitive%20Component%20Object%20Reference) (bSelfMoved :type Boolean) (HitLocation :type Vector :default "0, 0, 0") (HitNormal :type Vector :default "0, 0, 0") (NormalImpulse :type Vector :default "0, 0, 0") (Hit :type Hit%20Result%20Structure%20%28by%20ref%29))
  ;[1 1 1] Apply Damage to Player when Touching
  (Game|Damage|ApplyDamage Other (Variables|Default|GetTouchDamage) 0 0))

(event Game|Damage|EventAnyDamage
  (params (Damage :type Float%20%28single-precision%29) (DamageType :type Damage%20Type%20Object%20Reference) (InstigatedBy :type Controller%20Object%20Reference) (DamageCauser :type Actor%20Object%20Reference))
  ;[1 1 1] Damage & Decrease Health
  (if (not (== (Variables|Default|GetHealth) 0.0))
    (bind _output_get (Variables|Default|SetHealth (- (Variables|Default|GetHealth) Damage)))
    (if (<= _output_get 0.0)
      (Physics|SetSimulatePhysics (Variables|Character|GetMesh) true)
      (Components|DestroyComponent (Variables|Collision|GetCapsuleComponent))
      (CallFunction|EnemyKilled)
      (Utilities|FlowControl|Delay 3e+01)
      (Actor|DestroyActor))))

(fn ConstructionScript)